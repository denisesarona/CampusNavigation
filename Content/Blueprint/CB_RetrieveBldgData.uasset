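; CB_RetrieveBldgData is a Blueprint that queries a database for building records on BeginPlay.
; It opens a connection, runs a SELECT on buildingtbl with a literal 'BuildingName' filter, prints BuildingData's name without reading the result, then closes the connection.
; An else branch builds an INSERT from BuildingData through Format Text, without a connection wired.
; All branch conditions are constant true, so that insert and the failure messages never run.
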(event `self.ReceiveBeginPlay`
  (bind (_buildingid _inbldgtable _buildingname _buildingdescription _deptid _departmentname _isdepartment _amenitiesname _isamenities _keyfeatures _nofloors) (break `/Game/Blueprint/BS_BuildingInfo` (`self.BuildingData`)))
  (bind _connection (`/Game/Blueprint/ProjectFunctiions.CreateDatabaseConnection`))
  (if true
    (`/Game/Blueprint/ProjectFunctiions.DatabaseQuery` (`KismetTextLibrary.Conv_TextToString` (`|FormatText` "SELECT * FROM buildingtbl WHERE building_name='BuildingName'; \n")) _connection)
    (if true
      (`KismetSystemLibrary.PrintString` (`.BuildingName_2_3734DC734C14E93F1EDD06B06301048B` (break `/Game/Blueprint/BS_BuildingInfo` (`self.BuildingData`))))
      (`/Game/Blueprint/ProjectFunctiions.CloseDatabaseConnection` _connection)
      (if true
        (`KismetSystemLibrary.PrintString` "Connectuion Close")
        (else
          (`KismetSystemLibrary.PrintString` "fail to close")))
      (else
        (`/Game/Blueprint/ProjectFunctiions.DatabaseQuery` (`KismetTextLibrary.Conv_TextToString` (`|FormatText` "INSERT INTO buildingtbl (in_bldgtable, building_name, building_description, dept_id, department_name, is_department, amenities_name, is_amenities, key_features, no_floors) VALUES ('{InBldgTable}', '{BuildingName}', '{BuildingDescription}', '{DeptID}', '{DepartmentName}', '{IsDepartment}', '{AmenitiesName}', '{IsAmenities}', '{KeyFeatures}', '{NoFloors}');" _inbldgtable _buildingname _buildingdescription _deptid _departmentname _isdepartment _amenitiesname _isamenities _keyfeatures _nofloors)))
        (if true
          (`KismetSystemLibrary.PrintString` "Hello")
          (else
            (`KismetSystemLibrary.PrintString` "failed to insert")))))
    (else
      (`KismetSystemLibrary.PrintString` "Database connection failed!"))))